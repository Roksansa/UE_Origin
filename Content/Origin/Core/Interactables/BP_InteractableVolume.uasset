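; Interactable volume that toggles character buoyancy at a water surface.
; On BeginPlay it binds to the actor begin and end overlap events of its SurfaceWater reference.
; Overlapping OBaseCharacters get ChangeBuoyancyFromSurfaceVolume called with true on entry and false on exit.
; Both handlers print colored debug messages, including when the cast fails.
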(event Custom|EndOverlap
  (params (OverlappedActor :type Actor%20Object%20Reference) (OtherActor :type Actor%20Object%20Reference))
  ;[1 1 1] Overlap method for water surface. With debug info
  (bind _asobase_character (Utilities|Casting|CastToOBaseCharacter OtherActor)
    (:then
      (Development|PrintString "Hello Cast Successful endOverlap" true true "(R=0.000000,G=1.000000,B=0.284335,A=1.000000)")
      (Class|OBaseCharacter|ChangeBuoyancyfromSurfaceVolume _asobase_character false))
    (:CastFailed
      (Development|PrintString (Utilities|GetObjectName OverlappedActor) true true "(R=1.000000,G=0.609648,B=0.147550,A=1.000000)"))))

(event Custom|StartOverlap
  (params (OverlappedActor :type Actor%20Object%20Reference) (OtherActor :type Actor%20Object%20Reference))
  ;[1 1 1] Overlap method for water surface. With debug info
  (bind _asobase_character (Utilities|Casting|CastToOBaseCharacter OtherActor)
    (:then
      (Development|PrintString "Hello Cast Successful startOverlap" true true "(R=1.000000,G=0.196835,B=0.820312,A=1.000000)")
      (Class|OBaseCharacter|ChangeBuoyancyfromSurfaceVolume _asobase_character true))
    (:CastFailed
      (Development|PrintString "Hello fail cast"))))

(event EventBeginPlay
  ;[1 1 1] Overlap method for water surface. With debug info
  (Collision|BindEventtoOnActorBeginOverlap (Variables|Default|GetSurfaceWater) (delegate Custom|StartOverlap))
  (Collision|BindEventtoOnActorEndOverlap (Variables|Default|GetSurfaceWater) (delegate Custom|EndOverlap)))

(fn ConstructionScript)