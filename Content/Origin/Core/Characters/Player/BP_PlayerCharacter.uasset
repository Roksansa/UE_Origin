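; Player character Blueprint that changes the spring arm camera boom length when sprinting.
; It caches the spring arm's default length on BeginPlay.
; Sprint start plays a timeline that interpolates the arm from that default toward a sprint length, and sprint end reverses the same timeline to ease it back.
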(event EventOnSprintStart
  (bind _time (Timeline|Spring%20arm%20sprint%20timeline Play)
    (:Update
      (Variables|/Script/Engine.SpringArmComponent|SetTargetArmLength (Variables|Default|GetSpringArmComponent) (Math|Float|Lerp (Variables|Character|GetDefaultArmLength) (Variables|Character|GetSpringArmLength) _time)))))

(event EventOnSprintEnd
  (bind _time (Timeline|Spring%20arm%20sprint%20timeline Reverse)
    (:Update
      (Variables|/Script/Engine.SpringArmComponent|SetTargetArmLength (Variables|Default|GetSpringArmComponent) (Math|Float|Lerp (Variables|Character|GetDefaultArmLength) (Variables|Character|GetSpringArmLength) _time)))))

(event EventBeginPlay
  (Variables|Character|SetDefaultArmLength (Variables|/Script/Engine.SpringArmComponent|GetTargetArmLength (Variables|Default|GetSpringArmComponent))))

(fn ConstructionScript)